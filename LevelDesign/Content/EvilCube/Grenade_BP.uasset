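; Grenade Blueprint that knocks back and damages a ThirdPersonCharacter when it begins overlapping the Body component.
; It flattens and normalizes the character-to-Body direction, adds a fixed upward component, and scales it by LaunchVelocity for LaunchCharacter.
; The launch adds to existing velocity, then ApplyDamage deals the Damage value.
; A low-pitched explosion sound node exists but is disconnected, so it never plays.
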(event `self.body.OnComponentBeginOverlap`
  (params (OverlappedComponent :type "PrimitiveComponent Object Reference") (OtherActor :type "Actor Object Reference") (OtherComp :type "PrimitiveComponent Object Reference") (OtherBodyIndex :type Integer) (bFromSweep :type Boolean) (SweepResult :type "HitResult Structure (by ref)"))
  (bind _asthird_person_character (cast `/Game/ThirdPersonBP/Blueprints/ThirdPersonCharacter` OtherActor))
  (bind (_returnvalue_x _returnvalue_y) (`KismetMathLibrary.BreakVector` (`KismetMathLibrary.GetDirectionUnitVector` (`self.K2_GetActorLocation` _asthird_person_character) (`SceneComponent.K2_GetComponentLocation` (`self.body`)))))
  (bind (_returnvalue_x_2 _returnvalue_y_2) (`KismetMathLibrary.BreakVector` (`KismetMathLibrary.Normal` (`KismetMathLibrary.MakeVector` _returnvalue_x _returnvalue_y))))
  (`Character.LaunchCharacter` _asthird_person_character (* (`KismetMathLibrary.MakeVector` _returnvalue_x_2 _returnvalue_y_2 0.5) (`self.Launch Velocity`)) false false)
  (`GameplayStatics.ApplyDamage` _asthird_person_character (`self.Damage`)))

(fn `UserConstructionScript`)